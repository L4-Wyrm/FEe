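; Base spawner structure that periodically spawns random creatures around itself, skipped for preview placement.
; A looping timer rolls a spawn chance, and each success rolls again for an extra unique creature, both offset only toward positive X and Y.
; Authority loads tuning from INI after the timer starts, so its interval keeps the default.
; A sphere sized to the minimum radius destroys overlapping FEe skeletal, DodoRex and ZombieDodo creatures.
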(event `self.ReceiveBeginPlay`
  (if (not (`self.bIsPreviewStructure`))
    (`|ExecutionSequence`
      (:`then_0`
        (`KismetSystemLibrary.K2_SetTimer` null "EventInitSpawn" (`self.DelayBeforeSpawn`) true))
      (:`then_1`
        (`self.INIOptions`))
      (:`then_2`
        (`self.SetSphereRadius`)))))

(event `self.EggSpawnCollision.OnComponentBeginOverlap`
  (params (OtherActor :type "Actor Object Reference") (OtherComp :type "PrimitiveComponent Object Reference") (OtherBodyIndex :type Integer) (bFromSweep :type Boolean) (SweepResult :type "EngineTypes.HitResult Structure (by ref)"))
  (`self.FEeDinos` OtherActor))

(event `EventInitSpawn`
  (`self.SpawnRandomisedDino`))

(fn `FEeDinos`
  (params (DinoReference :type "Actor Object Reference"))
  (`|ExecutionSequence`
    (:`then_0`
      (bind _asmegaskelcarno_character_bp_fee_c (cast `/Game/Mods/FEe/Dinos/Carno/MegaSkelCarno_Character_BP_FEe` DinoReference)))
    (:`then_1`
      (bind _aszombiedodo_character_bp_fee_c (cast `/Game/Mods/FEe/Dinos/Dodo/ZombieDodo_Character_BP_FEe` DinoReference)))
    (:`then_2`
      (bind _asdodorex_character_bp_fee_c (cast `/Game/Mods/FEe/Dinos/DodoRex/DodoRex_Character_BP_FEe` DinoReference)))
    (:`then_3`
      (bind _asbone_gigant_character_bp_fee_c (cast `/Game/Mods/FEe/Dinos/Giganotosaurus/Bone_Gigant_Character_BP_FEe` DinoReference)))
    (:`then_4`
      (bind _asbone_quetz_character_bp_fee_c (cast `/Game/Mods/FEe/Dinos/Quetzalcoatlus/Bone_Quetz_Character_BP_FEe` DinoReference)))
    (:`then_5`
      (bind _asmegaskelraptor_character_bp_fee_c (cast `/Game/Mods/FEe/Dinos/Raptor/MegaSkelRaptor_Character_BP_FEe` DinoReference)))
    (:`then_6`
      (bind _asmegaskelrex_character_bp_fee_c (cast `/Game/Mods/FEe/Dinos/Rex/MegaSkelRex_Character_BP_FEe` DinoReference)))
    (:`then_7`
      (bind _asbone_sauropod_character_bp_fee_c (cast `/Game/Mods/FEe/Dinos/Sauropod/Bone_Sauropod_Character_BP_FEe` DinoReference)))
    (:`then_8`
      (bind _asbone_stego_character_bp_fee_c (cast `/Game/Mods/FEe/Dinos/Stego/Bone_Stego_Character_BP_FEe` DinoReference)))
    (:`then_9`
      (bind _asbone_trike_character_bp_fee_c (cast `/Game/Mods/FEe/Dinos/Trike/Bone_Trike_Character_BP_FEe` DinoReference))))
  (`self.K2_DestroyActor` _asmegaskelraptor_character_bp_fee_c)
  (`self.K2_DestroyActor` _asbone_quetz_character_bp_fee_c)
  (`self.K2_DestroyActor` _asbone_gigant_character_bp_fee_c)
  (`self.K2_DestroyActor` _asdodorex_character_bp_fee_c)
  (`self.K2_DestroyActor` _aszombiedodo_character_bp_fee_c)
  (`self.K2_DestroyActor` _asmegaskelcarno_character_bp_fee_c)
  (`self.K2_DestroyActor` _asmegaskelrex_character_bp_fee_c)
  (`self.K2_DestroyActor` _asbone_sauropod_character_bp_fee_c)
  (`self.K2_DestroyActor` _asbone_stego_character_bp_fee_c)
  (`self.K2_DestroyActor` _asbone_trike_character_bp_fee_c))

(fn `INIOptions`
  (`/Engine/EditorBlueprintResources/ActorMacros.Switch Has Authority`
    (:`Authority`
      (bind _asshootergamemode (cast `ShooterGameMode` (`GameplayStatics.GetGameMode`)))
      (`|ExecutionSequence`
        (:`then_0`
          (`ShooterGameMode.InitOptionFloat` _asshootergamemode "" (`self.SpawnerSettings`) (`self.SpawningChanceString`) (`self.SpawningChance`))
          (`ShooterGameMode.InitOptionFloat` _asshootergamemode "" (`self.SpawnerSettings`) (`self.MinSpawnRadiusString`) (`self.CollisionSphereMinRadius`))
          (`ShooterGameMode.InitOptionFloat` _asshootergamemode "" (`self.SpawnerSettings`) (`self.DelayBeforeSpawnString`) (`self.DelayBeforeSpawn`))
          (`ShooterGameMode.InitOptionFloat` _asshootergamemode "" (`self.SpawnerSettings`) (`self.SpawningChanceUniqueString`) (`self.SpawningChanceUnique`))
          (`ShooterGameMode.InitOptionFloat` _asshootergamemode "" (`self.SpawnerSettings`) (`self.MaxSpawnRadiusString`) (`self.CollisionSphereMaxRadius`)))
        (:`then_1`
          (bind _returnvalue (`ShooterGameMode.GetFloatOptionIni` _asshootergamemode (`self.SpawnerSettings`) (`self.SpawningChanceString`)))
          (set `self.SpawningChance` _returnvalue)
          (bind _returnvalue_2 (`ShooterGameMode.GetFloatOptionIni` _asshootergamemode (`self.SpawnerSettings`) (`self.MinSpawnRadiusString`)))
          (set `self.CollisionSphereMinRadius` _returnvalue_2)
          (bind _returnvalue_3 (`ShooterGameMode.GetFloatOptionIni` _asshootergamemode (`self.SpawnerSettings`) (`self.DelayBeforeSpawnString`)))
          (set `self.DelayBeforeSpawn` _returnvalue_3)
          (bind _returnvalue_4 (`ShooterGameMode.GetFloatOptionIni` _asshootergamemode (`self.SpawnerSettings`) (`self.SpawningChanceUniqueString`)))
          (set `self.SpawningChanceUnique` _returnvalue_4)
          (bind _returnvalue_5 (`ShooterGameMode.GetFloatOptionIni` _asshootergamemode (`self.SpawnerSettings`) (`self.MaxSpawnRadiusString`)))
          (set `self.CollisionSphereMaxRadius` _returnvalue_5))))))

(fn `SetSphereRadius`
  (`SphereComponent.SetSphereRadius` (`self.EggSpawnCollision`) (`self.CollisionSphereMinRadius`) true))

(fn `SpawnRandomisedDino`
  (bind _collisionsphereminradius (`self.CollisionSphereMinRadius`))
  (bind _collisionsphereminradius_2 (`self.CollisionSphereMinRadius`))
  (bind _creaturelist (`self.CreatureList`))
  (if (<= (`KismetMathLibrary.RandomFloat`) (`self.SpawningChance`))
    (`KismetArrayLibrary.Array_Shuffle` _creaturelist)
    (bind _returnvalue (`|SpawnActorFromClass` (`KismetArrayLibrary.Array_Get` _creaturelist (`KismetMathLibrary.RandomIntegerInRange` 0 (`KismetArrayLibrary.Array_LastIndex` (`self.CreatureList`)))) (`KismetMathLibrary.MakeTransform` (`KismetMathLibrary.MakeVector` (+ (.x (.location (`KismetMathLibrary.Conv_VectorToTransform` (`self.K2_GetActorLocation` self)))) (`KismetMathLibrary.RandomFloatInRange` _collisionsphereminradius_2 (+ _collisionsphereminradius_2 (`self.CollisionSphereMaxRadius`)))) (+ (.y (.location (`KismetMathLibrary.Conv_VectorToTransform` (`self.K2_GetActorLocation` self)))) (`KismetMathLibrary.RandomFloatInRange` _collisionsphereminradius (+ _collisionsphereminradius (`self.CollisionSphereMaxRadius`)))) (+ (.z (.location (`KismetMathLibrary.Conv_VectorToTransform` (`self.K2_GetActorLocation` self)))) 150.0)) (.rotation (`KismetMathLibrary.Conv_VectorToTransform` (`self.K2_GetActorLocation` self))) (.scale (`KismetMathLibrary.Conv_VectorToTransform` (`self.K2_GetActorLocation` self)))) true))
    (`|ExecutionSequence`
      (:`then_0`
        (if (not (`VictoryCore.IsShipping`))
          (if (`VictoryCore.IsPlayInEditor`)
            (bind _asprimaldinocharacter (cast `PrimalDinoCharacter` _returnvalue))
            (`PrimalDinoCharacter.BPUnstasis` _asprimaldinocharacter))))
      (:`then_1`
        (`self.SpawnRandomisedUniqueDino`)))))

(fn `SpawnRandomisedUniqueDino`
  (bind _collisionsphereminradius (`self.CollisionSphereMinRadius`))
  (bind _collisionsphereminradius_2 (`self.CollisionSphereMinRadius`))
  (bind _uniquecreaturelist (`self.UniqueCreatureList`))
  (if (<= (`KismetMathLibrary.RandomFloat`) (`self.SpawningChanceUnique`))
    (`KismetArrayLibrary.Array_Shuffle` _uniquecreaturelist)
    (bind _returnvalue (`|SpawnActorFromClass` (`KismetArrayLibrary.Array_Get` _uniquecreaturelist (`KismetMathLibrary.RandomIntegerInRange` 0 (`KismetArrayLibrary.Array_LastIndex` (`self.UniqueCreatureList`)))) (`KismetMathLibrary.MakeTransform` (`KismetMathLibrary.MakeVector` (+ (.x (.location (`KismetMathLibrary.Conv_VectorToTransform` (`self.K2_GetActorLocation` self)))) (`KismetMathLibrary.RandomFloatInRange` _collisionsphereminradius_2 (+ _collisionsphereminradius_2 (`self.CollisionSphereMaxRadius`)))) (+ (.y (.location (`KismetMathLibrary.Conv_VectorToTransform` (`self.K2_GetActorLocation` self)))) (`KismetMathLibrary.RandomFloatInRange` _collisionsphereminradius (+ _collisionsphereminradius (`self.CollisionSphereMaxRadius`)))) (+ (.z (.location (`KismetMathLibrary.Conv_VectorToTransform` (`self.K2_GetActorLocation` self)))) 150.0)) (.rotation (`KismetMathLibrary.Conv_VectorToTransform` (`self.K2_GetActorLocation` self))) (.scale (`KismetMathLibrary.Conv_VectorToTransform` (`self.K2_GetActorLocation` self)))) true))
    (if (not (`VictoryCore.IsShipping`))
      (if (`VictoryCore.IsPlayInEditor`)
        (bind _asprimaldinocharacter (cast `PrimalDinoCharacter` _returnvalue))
        (`PrimalDinoCharacter.BPUnstasis` _asprimaldinocharacter)))
    (else
      (`self.K2_DestroyActor` _returnvalue))))

(fn `UserConstructionScript`
  (`parent.UserConstructionScript`))