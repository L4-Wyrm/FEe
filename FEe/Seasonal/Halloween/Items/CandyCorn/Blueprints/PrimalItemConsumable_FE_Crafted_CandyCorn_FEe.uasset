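; Crafted Halloween candy corn consumable that gives a dino Buff_FestiveDinoColors, recoloring it and boosting speed.
; Item init rolls Primitive, Mastercraft or Ascendant quality and weighted-random dye colors, with a fixed rainbow set for Ascendant.
; Use replaces any existing buff; the server passes it tier-saturated colors, rerolling Ascendant ones with inverted weights to favor rare dyes.
; Icon saturation and tooltip speed follow quality, and non-Ascendant tooltips list region colors.
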(fn BPGetItemDescription
  (params (InDescription :type String) (bGetLongDescription :type Boolean) (ForPC :type Shooter%20Player%20Controller%20Object%20Reference))
  (bind _lines (LocalVariables|GetLines))
  (bind _lines_2 (LocalVariables|GetLines))
  (Utilities|Array|Clear _lines)
  (Utilities|Array|Add _lines InDescription)
  (Utilities|FlowControl|Sequence
    (:then_0
      (bind _percent (CallFunction|GetBuffSpeedPercentage))
      (Utilities|Array|Add (LocalVariables|GetLines) (Utilities|String|ToString(Text) (Utilities|Text|FormatText "Movement Speed: +{pct}%" (Utilities|Text|ToText(Float) _percent "HalfToEven" true 1 324 0 0)))))
    (:then_1
      (if (< (Math|Conversions|ToInteger(Byte) (Variables|Default|GetItemQualityIndex)) 5)
        (bind _returnvalue (Class|PrimalGameData|BPGetGameData))
        (for _index (range 0 5)
          (bind _returnvalue_2 (Class|PrimalItem|GetItemColorID _index))
          (bind _returnvalue_3 (Class|PrimalItem|StaticGetColorforItemColorID _returnvalue_2))
          (Utilities|Array|Add (LocalVariables|GetLines) (Utilities|String|ToString(Text) (Utilities|Text|FormatText "Region {region} : <RichColor Color=\"{color}\">{colorName}</>" (Utilities|Text|ToText(Integer) (+ _index 1)) (Utilities|Text|ToText(String) (Utilities|String|JoinStringArray (Utilities|Array|MakeArray (Utilities|String|ToString(Float) (.R (Utilities|Struct|BreakLinearColor _returnvalue_3))) (Utilities|String|ToString(Float) (.G (Utilities|Struct|BreakLinearColor _returnvalue_3))) (Utilities|String|ToString(Float) (.B (Utilities|Struct|BreakLinearColor _returnvalue_3))) "1") ", ")) (Utilities|Text|ToText(String) (CallFunction|GetDyeItemDescriptiveName _returnvalue _returnvalue_2))))))
        (else
          (Utilities|Array|Add _lines_2 "")
          (Utilities|Array|Add _lines_2 "The sweetest candy of them all!"))))
    (:then_2
      (return (Class|VictoryCore|JoinStringArraywithNewlines (LocalVariables|GetLines))))))

(fn BPPostAddBufftoGiveOwnerCharacter
  (params (OwnerCharacter :type Primal%20Character%20Object%20Reference) (Buff :type Primal%20Buff%20Object%20Reference))
  (Class|KismetSystemLibrary|IsRunningonServer Buff
    (:Yes
      (bind _asbuff_festivedinocolors_c (Utilities|Casting|CastToBuff_FestiveDinoColors Buff))
      (bind _returnvalue (Class|PrimalItem|GetItemDyeColors))
      (LocalVariables|SetDinoColors _returnvalue)
      (Utilities|FlowControl|Sequence
        (:then_0
          (switch int (Math|Conversions|ToInteger(Byte) (Variables|Default|GetItemQualityIndex))
            (:0
              ;[1 1 1] Primitive version: apply saturation value
              (for _index (range 0 5) :!label _label
                (Utilities|Array|SetArrayElem (LocalVariables|GetDinoColors) _index (Class|VictoryCore|ChangeSaturation (Utilities|Array|Get(acopy) (LocalVariables|GetDinoColors) _index) (Variables|Default|GetDinoSaturation_Primitive)) true)))
            (:1
              (goto _label))
            (:2
              (goto _label))
            (:3
              (goto _label))
            (:4
              ;[1 1 1] Mastercraft version: apply saturation value
              (for _index_2 (range 0 5)
                (Utilities|Array|SetArrayElem (LocalVariables|GetDinoColors) _index_2 (Class|VictoryCore|ChangeSaturation (Utilities|Array|Get(acopy) (LocalVariables|GetDinoColors) _index_2) (Variables|Default|GetDinoSaturation_Mastercraft)) true)))
            (:5
              ;[1 1 1] Ascendant version: generate colors now instead of pulling from the item color data; use inverted weights to get all the rare colors; apply saturation value
              (bind _weights (CallFunction|GetInvertedWeights))
              (for _index_3 (range 0 5)
                (bind _returnvalue_2 (Class|VictoryCore|GetWeightedRandomIndexfromArray _weights 0.0))
                (bind _returnvalue_3 (Class|PrimalItem|StaticGetColorforItemColorID (Class|PrimalItem|GetItemColorIDfromDyeItemID (Utilities|Array|Get(acopy) (Variables|Default|GetDyeItemIndices) _returnvalue_2))))
                (Utilities|Array|SetArrayElem (LocalVariables|GetDinoColors) _index_3 (Class|VictoryCore|ChangeSaturation _returnvalue_3 (Variables|Default|GetDinoSaturation_Ascendant)) true)))))
        (:then_1
          (Default|UpdateColorsfromItem _asbuff_festivedinocolors_c (LocalVariables|GetDinoColors) (Math|Conversions|ToInteger(Byte) (Variables|Default|GetItemQualityIndex))))))))

(fn BPInitItemColors
  (LocalVariables|SetDyeIDs (Variables|Default|GetFallbackColorIDs))
  (Utilities|FlowControl|Sequence
    (:then_0
      (LocalVariables|SetIsRainbow false)
      (LocalVariables|SetRand (Math|Random|RandomIntegerinRange 0 100))
      (if (< (LocalVariables|GetRand) (Math|Integer|Clamp(Integer) (- (- 100 (Variables|Default|GetPercentChance_Mastercraft)) (Variables|Default|GetPercentChance_Ascendant)) 0 100))
        (Class|PrimalItem|OverrideItemRating 0.0)
        (elif (< (LocalVariables|GetRand) (Math|Integer|Clamp(Integer) (- 100 (Variables|Default|GetPercentChance_Ascendant)) 0 100))
          (Class|PrimalItem|OverrideItemRating 8.0)
          (else
            (Class|PrimalItem|OverrideItemRating 15.0)
            (LocalVariables|SetIsRainbow true)
            (LocalVariables|SetDyeIDs (Utilities|Array|MakeArray 58 59 60 61 67 406))))))
    (:then_1
      (if (not (LocalVariables|GetIsRainbow))
        (for _index (range 0 5)
          (bind _returnvalue (Class|VictoryCore|GetWeightedRandomIndexfromArray (Variables|Default|GetDyeItemWeights) 0.0))
          (Utilities|Array|SetArrayElem (LocalVariables|GetDyeIDs) _index (Utilities|Array|Get(acopy) (Variables|Default|GetDyeItemIndices) _returnvalue) true))))
    (:then_2
      (return (Utilities|DyestoColorIDs (LocalVariables|GetDyeIDs))))))

(fn BPPreUseItem
  (bind _ownerinventory (Variables|Default|GetOwnerInventory))
  ;[1 1 1] Deactivate existing colorization buff so we can replace it with the new one
  (Utilities|IsValid _ownerinventory
    (:Is%20Valid
      (bind _asprimaldinocharacter (Utilities|Casting|CastToPrimalDinoCharacter (Components|GetOwner _ownerinventory)))
      (bind _returnvalue (Class|PrimalCharacter|GetBuff _asprimaldinocharacter (Variables|Default|GetBuffToGiveOwnerCharacter)))
      (Utilities|IsValid _returnvalue
        (:Is%20Valid
          (Class|PrimalBuff|BPDeactivate _returnvalue))))))

(fn GetInvertedWeights
  (Utilities|Array|Clear (LocalVariables|GetInverted))
  (Utilities|FlowControl|Sequence
    (:then_0
      (for (_array_element _array_index) (Variables|Default|GetDyeItemWeights)
        (Utilities|Array|SetArrayElem (LocalVariables|GetInverted) _array_index (/ 1.0 _array_element) true)))
    (:then_1
      (return (LocalVariables|GetInverted)))))

(fn GetDyeItemDescriptiveName
  (params (GameData :type Primal%20Game%20Data%20Object%20Reference) (A :type Integer))
  (LocalVariables|SetName "")
  (bind _returnvalue (Class|VictoryCore|GetClassDefaultObject (Utilities|Array|Get(acopy) (Variables|/Script/ShooterGame.PrimalGameData|GetMasterItemList GameData) (- A 1))))
  (bind _asprimalitem_dye (Utilities|Casting|CastToPrimalItem_Dye _returnvalue)
    (:then
      (LocalVariables|SetName (Variables|/Script/ShooterGame.PrimalItem|GetDescriptiveNameBase _asprimalitem_dye)))
    (:CastFailed
      _))
  (return (LocalVariables|GetName)))

(fn BPInitIconMaterial
  (bind _array (Utilities|Array|MakeArray "Color0_RedIntensity" "Color1_GreenIntensity" "Color2_BlueIntensity" "Color3_YellowIntensity" "Color4_CyanIntensity" "Color5_MagentaIntensity"))
  (bind _itemiconmaterial (Variables|Default|GetItemIconMaterial))
  (Utilities|IsValid (Variables|Default|GetItemIconMaterial)
    (:Is%20Valid
      (switch int (Math|Conversions|ToInteger(Byte) (Variables|Default|GetItemQualityIndex))
        (:0
          (for _array_element _array :!label _label
            (Rendering|Material|SetScalarParameterValue _itemiconmaterial _array_element (Variables|Default|GetIconSaturation_Primitive) :!class /Script/Engine.MaterialInstanceDynamic)))
        (:1
          (goto _label))
        (:2
          (goto _label))
        (:3
          (goto _label))
        (:4
          (for _array_element_2 _array
            (Rendering|Material|SetScalarParameterValue _itemiconmaterial _array_element_2 (Variables|Default|GetIconSaturation_Mastercraft) :!class /Script/Engine.MaterialInstanceDynamic)))
        (:5
          (Rendering|Material|SetTextureParameterValue _itemiconmaterial "Albedo Map" "/Game/PrimalEarth/Environment/Seasonal/Halloween/CandyCorn/Icon/HUD_Event_Halloween_BC.HUD_Event_Halloween_BC")
          (for _array_element_3 _array
            (Rendering|Material|SetScalarParameterValue _itemiconmaterial _array_element_3 (Variables|Default|GetIconSaturation_Ascendant) :!class /Script/Engine.MaterialInstanceDynamic))
          (for _index (range 0 5)
            (Rendering|Material|SetScalarParameterValue _itemiconmaterial (Utilities|String|StringToName (Utilities|String|Append "UsingColor" (Utilities|String|ToString(Integer) _index))) 0.0 :!class /Script/Engine.MaterialInstanceDynamic)
            (Rendering|Material|SetScalarParameterValue _itemiconmaterial (Utilities|String|StringToName (Utilities|String|Append "UsingColorizedColor" (Utilities|String|ToString(Integer) _index))) 0.0 :!class /Script/Engine.MaterialInstanceDynamic)))))))

(fn GetBuffSpeedPercentage
  (LocalVariables|SetSpeedPct 5.0)
  (Utilities|FlowControl|Sequence
    (:then_0
      (bind _returnvalue (Class|VictoryCore|GetClassDefaultObject (Variables|Default|GetBuffToGiveOwnerCharacter)))
      (bind _asbuff_festivedinocolors_c (Utilities|Casting|CastToBuff_FestiveDinoColors _returnvalue))
      (switch int (Math|Conversions|ToInteger(Byte) (Variables|Default|GetItemQualityIndex))
        (:0
          (LocalVariables|SetSpeedPct (* (- (Variables|/Script/ShooterGame.PrimalBuff|GetUnsubmergedMaxSpeedModifier _asbuff_festivedinocolors_c) 1.0) 1e+02) :!label _label))
        (:1
          (goto _label))
        (:2
          (goto _label))
        (:3
          (goto _label))
        (:4
          (LocalVariables|SetSpeedPct (* (- (Variables|/Game/PrimalEarth/CoreBlueprints/Buffs/Buff_FestiveDinoColors.Buff_FestiveDinoColors_C|GetSpeedMultiplier_Mastercraft _asbuff_festivedinocolors_c) 1.0) 1e+02)))
        (:5
          (LocalVariables|SetSpeedPct (* (- (Variables|/Game/PrimalEarth/CoreBlueprints/Buffs/Buff_FestiveDinoColors.Buff_FestiveDinoColors_C|GetSpeedMultiplier_Ascendant _asbuff_festivedinocolors_c) 1.0) 1e+02)))))
    (:then_1
      (return (Math|Float|Clamp(Float) (LocalVariables|GetSpeedPct) 0.0 1e+02)))))