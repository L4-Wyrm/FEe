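; Halloween candy corn buff that recolors a dino with colors passed from the item and sets its movement speed modifiers from item quality.
; The server multicasts colors and quality, and clients refresh colorization only when the colors differ.
; BPDinoRefreshColorization substitutes the stored six-color set for the dino's own.
; Delayed timers from BeginPlay and BPSetupForInstigator re-multicast stored values after save loads or unstasis.
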(event Custom|UpdateColorsFromItem
  (params (ItemColors :type Array%20of%20Linear%20Color%20Structures) (ItemQuality :type Integer))
  ;[1 1 1] Called from the item to pass in its colors to this buff
  (Class|KismetSystemLibrary|IsRunningonServer
    (:Yes
      (Variables|Default|SetGeneratedColors ItemColors false)
      (if (< (Class|VictoryCore|TimeSinceNetwork (Class|Actor|GetWorld) (Variables|Default|GetBuffStartTime)) 1.0)
        (Utilities|FlowControl|Delay 0.5))
      (CallFunction|MultiUpdateColors ItemColors ItemQuality))))

(event Custom|MultiUpdateColors
  (params (Colors :type Array%20of%20Linear%20Color%20Structures) (ItemQuality :type Integer))
  (bind _speedmult (Utilities|QualitytoSpeedMult ItemQuality))
  ;[1 1 1] Multicast for initial color syncing
  (Class|KismetSystemLibrary|IsRunningonServer
    (:Yes
      (Variables|Default|SetGeneratedColors Colors false :!label _label)
      (Variables|Default|SetCandyQualityLevel ItemQuality)
      (Utilities|FlowControl|Sequence
        (:then_0
          (Class|KismetSystemLibrary|CanRunCosmeticEvents
            (:Yes
              (bind _asprimaldinocharacter (Utilities|Casting|CastToPrimalDinoCharacter (Variables|Default|GetInstigator)))
              (Class|PrimalDinoCharacter|RefreshColorization _asprimaldinocharacter true))))
        (:then_1
          (Variables|Default|SetSubmergedMaxSpeedModifier _speedmult)
          (Variables|Default|SetUnsubmergedMaxSpeedModifier _speedmult))))
    (:No
      (bind _equal (CallFunction|AreColorArraysEqual (Variables|Default|GetGeneratedColors) Colors))
      (if (not _equal)
        (goto _label)))))

(event Custom|MultiUpdateAfterLoadSave
  (params (Colors :type Array%20of%20Linear%20Color%20Structures) (CandyQuality :type Integer))
  (bind _speedmult (Utilities|QualitytoSpeedMult CandyQuality))
  ;[1 1 1] Delayed multicast to sync colors after loading a save game
  (Utilities|FlowControl|Sequence
    (:then_0
      (Variables|Default|SetSubmergedMaxSpeedModifier _speedmult)
      (Variables|Default|SetUnsubmergedMaxSpeedModifier _speedmult))
    (:then_1
      (Class|KismetSystemLibrary|IsRunningonServer
        (:Yes
          (Variables|Default|SetGeneratedColors Colors false :!label _label)
          (Class|KismetSystemLibrary|CanRunCosmeticEvents
            (:Yes
              (bind _asprimaldinocharacter (Utilities|Casting|CastToPrimalDinoCharacter (Variables|Default|GetInstigator)))
              (Class|PrimalDinoCharacter|RefreshColorization _asprimaldinocharacter true))))
        (:No
          (bind _equal (CallFunction|AreColorArraysEqual (Variables|Default|GetGeneratedColors) Colors))
          (if (not _equal)
            (goto _label)))))))

(event Custom|DelayedPostLoadUpdate
  ;[1 1 1] Delayed multicast to sync colors after loading a save game
  (Class|KismetSystemLibrary|IsRunningonServer
    (:Yes
      (CallFunction|MultiUpdateAfterLoadSave (Variables|Default|GetGeneratedColors) (Variables|Default|GetCandyQualityLevel)))))

(event EventBeginPlay
  ;[1 1 1] Only need to refresh on BeginPlay if we already have colors (which means it's being loaded from a savegame or unstasised dino
  (|CallParentFunction)
  (if (> (Utilities|Array|Length (Variables|Default|GetGeneratedColors)) 0)
    (Class|KismetSystemLibrary|CanRunCosmeticEvents
      (:Yes
        (bind _asprimaldinocharacter (Utilities|Casting|CastToPrimalDinoCharacter (Variables|Default|GetInstigator)))
        (Class|PrimalDinoCharacter|RefreshColorization _asprimaldinocharacter true))
      (:No
        (Class|KismetSystemLibrary|IsRunningonServer
          (:Yes
            (Utilities|Time|SetTimerbyFunctionName self "DelayedPostLoadUpdate" 3.0)))))))

(fn ConstructionScript)

(fn BPDinoRefreshColorization
  (params (DinoColors :type Array%20of%20Linear%20Color%20Structures))
  (bind _generatedcolors (Variables|Default|GetGeneratedColors))
  (LocalVariables|SetCol DinoColors)
  (Utilities|FlowControl|Sequence
    (:then_0
      (if (== (Utilities|Array|Length _generatedcolors) 6)
        (LocalVariables|SetCol _generatedcolors)))
    (:then_1
      (return (LocalVariables|GetCol)))))

(fn BPSetupforInstigator
  (params (ForInstigator :type Actor%20Object%20Reference))
  (Class|KismetSystemLibrary|IsRunningonServer
    (:Yes
      (if (> (Utilities|Array|Length (Variables|Default|GetGeneratedColors)) 0)
        (Utilities|Time|SetTimerbyFunctionName self "DelayedPostLoadUpdate" 5.0)))))

(fn AreColorArraysEqual
  (params (A :type Array%20of%20Linear%20Color%20Structures) (B :type Array%20of%20Linear%20Color%20Structures))
  (bind _returnvalue (Utilities|Array|Length B))
  (Utilities|FlowControl|Sequence
    (:then_0
      (if (== (Utilities|Array|Length A) _returnvalue)
        (LocalVariables|SetSameColors true)
        (bind _index (Utilities|FlowControl|ForLoopwithBreak 0 (- _returnvalue 1) :!label _label)
          (:LoopBody
            (if (not (Class|KismetMathLibrary|NearlyEqualVectorVector (Math|Conversions|ToVector(LinearColor) (Utilities|Array|Get(acopy) A _index)) (Math|Conversions|ToVector(LinearColor) (Utilities|Array|Get(acopy) B _index)) 0.01))
              (LocalVariables|SetSameColors false)
              (goto _label Break))))
        (else
          (LocalVariables|SetSameColors false))))
    (:then_1
      (return (LocalVariables|GetSameColors)))))